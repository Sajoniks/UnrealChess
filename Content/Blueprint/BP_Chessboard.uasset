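; Chessboard Blueprint that visually plays out chess moves on piece actors in response to move and castling events.
; Normal moves cache the involved pieces, then a timeline lerps the mover between square locations with a height-scaled vertical offset.
; When it finishes, a sound plays and any captured or en passant piece is hidden rather than destroyed.
; Castling skips animation, teleporting both pieces and playing the same sound.
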(event EventOnCastlingMove
  (params (King :type Tile%20Object%20Reference) (NewKing :type Tile%20Object%20Reference) (Piece :type Tile%20Object%20Reference) (NewPiece :type Tile%20Object%20Reference))
  (|CastlingMove King Piece NewKing NewPiece))

(event EventOnMove
  (params (From :type Tile%20Object%20Reference) (To :type Tile%20Object%20Reference) (EnPas :type Tile%20Object%20Reference) (Move :type Chess%20Move%20Structure%20%28by%20ref%29))
  (|MoveAnimation From To EnPas Move))

(fn ConstructionScript)