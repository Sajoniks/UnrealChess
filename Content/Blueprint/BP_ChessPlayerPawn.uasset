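; BP_ChessPlayerPawn is the player pawn for a chess game, providing an orbit-style camera on a spring arm.
; Mouse X and Y drive controller yaw and pitch.
; The mouse wheel steps the arm length within min and max limits, with wheel down shortening it and wheel up lengthening it.
; On BeginPlay, a locally controlled pawn limits the pitch range through the player camera manager.
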(event EventBeginPlay
  (bind _returnvalue (Game|GetPlayerCameraManager 0))
  ;[1 1 1] Set angle constraints
  (if (Pawn|IsLocallyControlled)
    (Variables|/Script/Engine.PlayerCameraManager|SetViewPitchMin _returnvalue -5e+01)
    (Variables|/Script/Engine.PlayerCameraManager|SetViewPitchMax _returnvalue 3e+01)))

(event Input|MouseEvents|MouseX
  (params (AxisValue :type Float%20%28single-precision%29))
  (Pawn|Input|AddControllerYawInput AxisValue))

(event Input|MouseEvents|MouseY
  (params (AxisValue :type Float%20%28single-precision%29))
  (Pawn|Input|AddControllerPitchInput AxisValue))

(event Input|MouseEvents|MouseWheelUp
  (params (Key :type Key%20Structure :default "None"))
  (bind _springarm (Variables|Default|GetSpringArm))
  (:Pressed
    (Variables|/Script/Engine.SpringArmComponent|SetTargetArmLength _springarm (Math|Float|Clamp(Float) (+ (Variables|/Script/Engine.SpringArmComponent|GetTargetArmLength _springarm) (Variables|Default|GetArmZoomStep)) (Variables|Default|GetMinArmLength) (Variables|Default|GetMaxArmLength)))))

(event Input|MouseEvents|MouseWheelDown
  (params (Key :type Key%20Structure :default "None"))
  (bind _springarm (Variables|Default|GetSpringArm))
  (:Pressed
    (Variables|/Script/Engine.SpringArmComponent|SetTargetArmLength _springarm (Math|Float|Clamp(Float) (- (Variables|/Script/Engine.SpringArmComponent|GetTargetArmLength _springarm) (Variables|Default|GetArmZoomStep)) (Variables|Default|GetMinArmLength) (Variables|Default|GetMaxArmLength)))))

(fn ConstructionScript)