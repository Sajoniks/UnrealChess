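; Game mode for single-controller chess, where one player controller alternately plays White and Black.
; On begin play it spawns the chessboard and binds to its player-move event.
; On login it gathers the placed player pawns, possesses the White one and sets White as the moving side.
; Each move flips the controller's side and possesses the other pawn, relying on the found array order for color.
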(event Custom|OnMove
  (bind _return_value (CallFunction|GetChessPlayerController))
  (switch Utilities|FlowControl|Switch|SwitchonEPieceColor (Class|ChessPlayerController|GetSide _return_value)
    (:White
      (Class|ChessPlayerController|SetSide _return_value "Black")
      ;[1 1 1] Possess black pawn
      (Pawn|Possess (Game|GetPlayerController 0) (Utilities|Array|Get(acopy) (Variables|Default|GetPlayerPawns))))
    (:Black
      (Class|ChessPlayerController|SetSide _return_value "White")
      ;[1 1 1] Possess white pawn
      (Pawn|Possess (Game|GetPlayerController 0) (Utilities|Array|Get(acopy) (Variables|Default|GetPlayerPawns) 1)))))

(event EventBeginPlay
  (bind _returnvalue (Game|SpawnActorfromClass "/Game/Blueprint/BP_Chessboard.BP_Chessboard_C" (Math|Transform|MakeTransform "0, 0, 0") "AlwaysSpawn" (Game|GetGameState) 0))
  (bind _output_get (Variables|Default|SetChessboard _returnvalue))
  (EventDispatchers|AssignOnPlayerMove _output_get (delegate Custom|OnMove)))

(event EventPostLogin
  (params (NewPlayer :type Player%20Controller%20Object%20Reference))
  ;[1 1 1] Posses player
  (CallFunction|FindPlayerPawns)
  (Pawn|Possess NewPlayer (Utilities|Array|Get(acopy) (Variables|Default|GetPlayerPawns) 1))
  (bind _asbp_chess_player_controller (Utilities|Casting|CastToBP_ChessPlayerController NewPlayer))
  (Class|ChessPlayerController|SetSide _asbp_chess_player_controller "White") ; Set player piece color
  (Class|ChessGameState|SetMovingSide (CallFunction|GetChessGameState) "White"))

(fn ConstructionScript)

(fn FindPlayerPawns
  (bind _outactors (Actor|GetAllActorsOfClass "/Game/Blueprint/BP_ChessPlayerPawn.BP_ChessPlayerPawn_C"))
  (Variables|Default|SetPlayerPawns _outactors))