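; Chess game mode that sets up the board and assigns players to pawns and sides as they join.
; BeginPlay spawns BP_Chessboard at the world origin, owned by the GameState.
; PostLogin gathers the level's BP_ChessPlayerPawn actors, possesses one by join order, and sets the controller's side: first player Black, second White.
; When the second player joins, the game state's moving side is set to White.
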(event EventBeginPlay
  (bind _returnvalue (Game|SpawnActorfromClass "/Game/Blueprint/BP_Chessboard.BP_Chessboard_C" (Math|Transform|MakeTransform "0, 0, 0") "AlwaysSpawn" (Game|GetGameState) 0))
  (Variables|Default|SetChessboard _returnvalue))

(event EventPostLogin
  (params (NewPlayer :type Player%20Controller%20Object%20Reference))
  (CallFunction|FindPlayerPawns)
  ;[1 1 1] Posses players
  (bind _returnvalue (Class|GameModeBase|GetNumPlayers))
  (Pawn|Possess NewPlayer (Utilities|Array|Get(acopy) (Variables|Default|GetPlayerPawns) (- _returnvalue 1)))
  (bind _asbp_chess_player_controller (Utilities|Casting|CastToBP_ChessPlayerController NewPlayer))
  (Class|ChessPlayerController|SetSide _asbp_chess_player_controller (Utilities|Select :Index (- _returnvalue 1) :Option%200 "Black" :Option%201 "White")) ; Set player piece color
  (if (== (- _returnvalue 1) 1)
    (Class|ChessGameState|SetMovingSide (CallFunction|GetChessGameState) "White")))

(fn ConstructionScript)

(fn FindPlayerPawns
  (bind _outactors (Actor|GetAllActorsOfClass "/Game/Blueprint/BP_ChessPlayerPawn.BP_ChessPlayerPawn_C"))
  (Variables|Default|SetPlayerPawns _outactors))